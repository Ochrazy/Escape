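; EscapeGameMode is the game mode Blueprint that handles level progression through an OpenNextLevel event.
; It derives the next level number from the last character of the current level name, so only a single digit is read.
; If that number exceeds the LevelCount on EscapeGameInstance, it opens "Mars"; otherwise it opens "Level" plus the number.
; Either load follows a short delay.
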(event `self.ReceiveBeginPlay`)

(event `OpenNextLevel`
  (bind _returnvalue (`GameplayStatics.GetCurrentLevelName` true))
  (bind _asescape_game_instance (cast `/Game/Blueprints/EscapeGameInstance` (`GameplayStatics.GetGameInstance`)))
  (bind _returnvalue_2 (+ (`KismetStringLibrary.Conv_StringToInt` (`KismetStringLibrary.GetSubstring` _returnvalue (- (`KismetStringLibrary.Len` _returnvalue) 1))) 1))
  (if (< (`/Game/Blueprints/EscapeGameInstance.LevelCount` _asescape_game_instance) _returnvalue_2)
    (`KismetSystemLibrary.Delay` 0.2)
    (`GameplayStatics.OpenLevel` "Mars")
    (else
      (`KismetSystemLibrary.Delay` 0.2)
      (`GameplayStatics.OpenLevel` (`KismetStringLibrary.Conv_StringToName` (`KismetStringLibrary.BuildString_Int` "Level" "" _returnvalue_2))))))

(fn `UserConstructionScript`)