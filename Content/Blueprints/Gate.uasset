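; Gate actor that ends a level when a BlockGoal hits it, letting the block escape.
; The hit disables actor collision and touch events, stops the block following, plays the controller's UI animation and swings the gate open.
; Tick watches yaw thresholds to reverse RotatingMovement into a slower closing swing, then stops it and asks EscapeGameMode to open the next level.
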(event `self.StaticMesh.OnComponentHit`
  (params (HitComponent :type "PrimitiveComponent Object Reference") (OtherActor :type "Actor Object Reference") (OtherComp :type "PrimitiveComponent Object Reference") (NormalImpulse :type "Vector Structure") (Hit :type "HitResult Structure (by ref)"))
  (bind _asblock_goal (cast `/Game/Blueprints/BlockGoal` OtherActor))
  (`self.SetActorEnableCollision` false)
  (`|ExecutionSequence`
    (:`then_0`
      ;[1 1 1] Stop the Goal Block from following the Touch/Cursor
      (set `PlayerController.bEnableTouchEvents` false (`GameplayStatics.GetPlayerController` 0))
      (`/Game/Blueprints/Block.StopFollowing` _asblock_goal)
      (set `/Game/Blueprints/BlockGoal.bIsEscaping` true _asblock_goal))
    (:`then_1`
      ;[1 1 1] Play UI Animation
      (bind _asescape_player_controller (cast `/Game/Blueprints/EscapePlayerController` (`GameplayStatics.GetPlayerController` 0)))
      (`/Game/Blueprints/EscapePlayerController.PlayUIAnimation` _asescape_player_controller))
    (:`then_2`
      ;[1 1 1] Open Gate
      (set `RotatingMovementComponent.RotationRate` (struct :`Yaw` 360.0) (`self.RotatingMovement`))
      (`self.SetActorTickEnabled` true))))

(event `self.ReceiveTick`
  (params (DeltaSeconds :type "Float (single-precision)"))
  (if (`self.bIsClosing`)
    ;[1 1 1] Check if Gate is closed
    (if (>= (.yaw (`self.K2_GetActorRotation`)) 0.0)
      (set `RotatingMovementComponent.RotationRate` (struct) (`self.RotatingMovement`))
      ;[1 1 1] Open Next Level
      (bind _asescape_game_mode (cast `/Game/Blueprints/EscapeGameMode` (`GameplayStatics.GetGameMode`)))
      (`/Game/Blueprints/EscapeGameMode.OpenNextLevel` _asescape_game_mode))
    (else
      ;[1 1 1] Close Gate
      (if (>= (.yaw (`self.K2_GetActorRotation`)) -45.0)
        (set `RotatingMovementComponent.RotationRate` (struct :`Yaw` -50.0) (`self.RotatingMovement`))
        (set `self.bIsClosing` true)))))

(fn `UserConstructionScript`)